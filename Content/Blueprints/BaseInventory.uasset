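; BaseInventory is an Actor Blueprint that stores picked-up items as slots with stack counts, under a weight limit.
; AddItemToInventory tops up a same-name partial stack for stackable items, otherwise appending a slot if space remains.
; The weight check sums one ItemWeight per slot, ignoring stack count, and is skipped when topping up.
; Item actors are hidden with collision disabled, even when the inventory is full.
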(fn `AddItemToInventory`
  (params (InItem :type "/Game/Blueprints/BaseItem Object Reference"))
  (returns (index :type Integer))
  (locals (IndexAdded :type Integer))
  (bind _indexadded (`local.IndexAdded`))
  (`self.CanItStack` InItem
    (:`true`
      (bind _index (`self.HasPartialStack` InItem)
        (:`true`
          (set `local.IndexAdded` _index))
        (:`false`
          (`self.HasInventorySpace` :!label _label
            (:`true`
              (bind _returnvalue (`KismetArrayLibrary.Array_Add` (`self.ItemList`) (make `/Game/Blueprints/InventorySlot` InItem 1)))
              (set `local.IndexAdded` _returnvalue))))))
    (:`false`
      (goto _label)))
  (`KismetSystemLibrary.PrintString` (`KismetStringLibrary.BuildString_Int` "" "Item added at: " _indexadded))
  (`self.SetActorHiddenInGame` InItem true)
  (`self.SetActorEnableCollision` InItem false)
  (return _indexadded))

(fn `UserConstructionScript`)