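; AgroCheck is an AI tick Blueprint, likely a behavior tree service, that finds visible targets for enemies to follow.
; Each tick it sphere-traces around the pawn for desired object types, ignoring AI_Enemy actors, then line-traces to each hit on the Camera channel.
; Visible hits set TargetToFollow and TargetLocation; blocked hits clear only TargetToFollow, so the last hit processed decides the target.
; The Enemy_AI_CON controller is cached on first use.
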(event `self.ReceiveTickAI`
  (params (OwnerController :type "AIController Object Reference") (ControlledPawn :type "Pawn Object Reference") (DeltaSeconds :type "Float (single-precision)"))
  (bind _returnvalue (`Actor.K2_GetActorLocation` (`Controller.K2_GetPawn` (`self.AI_CON_Ref`))))
  (if (not (!= (`self.AI_CON_Ref`) null))
    (bind _asenemy_ai_con (cast `/Game/Blueprints/Enemy/Enemy_AI_CON` OwnerController))
    (set `self.AI_CON_Ref` _asenemy_ai_con))
  (bind _outactors (`GameplayStatics.GetAllActorsOfClass` "/Game/Blueprints/Enemy/AI_Enemy.AI_Enemy_C"))
  (set `self.myLocation` _returnvalue)
  (bind _outhits (`KismetSystemLibrary.SphereTraceMultiForObjects` _returnvalue (+ _returnvalue (0.0 0.0 15.0)) 2000.0 (`self.DesiredObjectTypes`) false _outactors))
  (for _array_element _outhits
    (bind (_bblockinghit _binitialoverlap _time _location _impactpoint _normal _impactnormal _physmat _hitactor) (`GameplayStatics.BreakHitResult` _array_element))
    (bind _outhit (`KismetSystemLibrary.LineTraceSingle` (`self.myLocation`) (`Actor.K2_GetActorLocation` _hitactor) "TraceTypeQuery2" false _outactors))
    (bind (_bblockinghit_2 _binitialoverlap_2 _time_2 _location_2 _impactpoint_2 _normal_2 _impactnormal_2 _physmat_2 _hitactor_2) (`GameplayStatics.BreakHitResult` _outhit))
    (if (== _hitactor_2 _hitactor)
      (`BTFunctionLibrary.SetBlackboardValueAsObject` (`self.TargetToFollow`) _hitactor_2)
      (`BTFunctionLibrary.SetBlackboardValueAsVector` (`self.TargetLocation`) (`Actor.K2_GetActorLocation` _hitactor_2))
      (else
        (`BTFunctionLibrary.SetBlackboardValueAsObject` (`self.TargetToFollow`))))))