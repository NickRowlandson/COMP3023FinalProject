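; Behavior tree task that moves an enemy's controlled pawn to the actor stored in the TargetToFollow blackboard key.
; It casts the owner to Enemy_AI_CON on first use, caches that reference, then runs AIMoveTo with a small acceptance radius.
; The task finishes successfully when the move succeeds; a failed move or failed cast never calls FinishExecute.
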(event `self.ReceiveExecute`
  (params (OwnerActor :type "Actor Object Reference"))
  (if (not (!= (`self.AI_CON_Ref`) null))
    (bind _asenemy_ai_con (cast `/Game/Blueprints/Enemy/Enemy_AI_CON` OwnerActor))
    (set `self.AI_CON_Ref` _asenemy_ai_con))
  (`|AIMoveTo` (`Controller.K2_GetPawn` (`self.AI_CON_Ref`)) (0.0 0.0 0.0) (`BTFunctionLibrary.GetBlackboardValueAsActor` (`self.TargetToFollow`)) 50.0
    (:`OnSuccess`
      (`self.FinishExecute` true))))