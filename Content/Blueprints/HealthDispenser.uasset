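; HealthDispenser is an interactable actor that restores the player character's health when E is pressed.
; Overlapping its Box enables input for player controller 0, and leaving disables it, without checking which actor overlapped.
; On E it takes the first ThirdPersonCharacter found in the world and adds a fixed amount to CharacterHealth, capped at 100.
; It has no cooldown or use limit.
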(event `self.Box.OnComponentBeginOverlap`
  (params (OverlappedComponent :type "PrimitiveComponent Object Reference") (OtherActor :type "Actor Object Reference") (OtherComp :type "PrimitiveComponent Object Reference") (OtherBodyIndex :type Integer) (bFromSweep :type Boolean) (SweepResult :type "HitResult Structure (by ref)"))
  (`self.EnableInput` (`GameplayStatics.GetPlayerController` 0)))

(event `self.Box.OnComponentEndOverlap`
  (params (OverlappedComponent :type "PrimitiveComponent Object Reference") (OtherActor :type "Actor Object Reference") (OtherComp :type "PrimitiveComponent Object Reference") (OtherBodyIndex :type Integer))
  (`self.DisableInput` (`GameplayStatics.GetPlayerController` 0)))

(event `Key|E`
  (params (Key :type "Key Structure" :default "AnyKey"))
  (:`Pressed`
    (bind _outactors (`GameplayStatics.GetAllActorsOfClass` "/Game/ThirdPersonBP/Blueprints/ThirdPersonCharacter.ThirdPersonCharacter_C"))
    (bind _item (`KismetArrayLibrary.Array_Get` _outactors))
    (bind _characterhealth (`/Game/ThirdPersonBP/Blueprints/ThirdPersonCharacter.CharacterHealth` _item))
    (if (> (+ _characterhealth 25) 100)
      (set `/Game/ThirdPersonBP/Blueprints/ThirdPersonCharacter.CharacterHealth` 100 _item)
      (elif (not (>= _characterhealth 100))
        (set `/Game/ThirdPersonBP/Blueprints/ThirdPersonCharacter.CharacterHealth` (+ _characterhealth 25) _item)))))

(fn `UserConstructionScript`)