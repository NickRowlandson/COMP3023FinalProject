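; Interactive fire actor that the player fuels with wood and toggles on and off, starting unlit.
; While input is enabled by overlap, F moves a Wood stack from the backpack into FireWood and E toggles particles, audio and damage collision.
; A restarting BurningWood timeline consumes one wood per cycle and extinguishes the fire when empty.
; Overlapping the damage component subtracts health from the first ThirdPersonCharacter found, whatever actor overlapped.
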(event `self.TakeDamage.OnComponentBeginOverlap`
  (params (OverlappedComponent :type "PrimitiveComponent Object Reference") (OtherActor :type "Actor Object Reference") (OtherComp :type "PrimitiveComponent Object Reference") (OtherBodyIndex :type Integer) (bFromSweep :type Boolean) (SweepResult :type "HitResult Structure (by ref)"))
  ;[1 1 1] Remove health from character on overlap
  (bind _outactors (`GameplayStatics.GetAllActorsOfClass` "/Game/ThirdPersonBP/Blueprints/ThirdPersonCharacter.ThirdPersonCharacter_C"))
  (bind _item (`KismetArrayLibrary.Array_Get` _outactors))
  (set `/Game/ThirdPersonBP/Blueprints/ThirdPersonCharacter.CharacterHealth` (+ (`/Game/ThirdPersonBP/Blueprints/ThirdPersonCharacter.CharacterHealth` _item) -25) _item))

(event `self.ReceiveActorBeginOverlap`
  (params (OtherActor :type "Actor Object Reference"))
  ;[1 1 1] Enable input
  (`self.EnableInput` (`GameplayStatics.GetPlayerController` 0)))

(event `self.ReceiveActorEndOverlap`
  (params (OtherActor :type "Actor Object Reference"))
  ;[1 1 1] Enable input
  (`self.DisableInput` (`GameplayStatics.GetPlayerController` 0)))

(event `noWood`
  ;[1 1 1] Turn off/on fire
  (`ActorComponent.Deactivate` (`self.P_Fire`) :!label _label)
  (`ActorComponent.Deactivate` (`self.Audio`))
  (`ActorComponent.Deactivate` (`self.P_Smoke`))
  (`PrimitiveComponent.SetCollisionEnabled` (`self.TakeDamage`) "NoCollision")
  (set `self.fireBoolean` false))

(event `self.ReceiveBeginPlay`
  (goto _label))

(event `Key|E`
  (params (Key :type "Key Structure" :default "AnyKey"))
  (:`Pressed`
    ;[1 1 1] Turn off/on fire
    (if (`self.fireBoolean`)
      (goto _label)
      (elif (> (`self.fireWood`) 0)
        (`ActorComponent.Activate` (`self.P_Fire`) false)
        (`ActorComponent.Activate` (`self.Audio`) false)
        (`ActorComponent.Activate` (`self.P_Smoke`) false)
        (`PrimitiveComponent.SetCollisionEnabled` (`self.TakeDamage`) "QueryAndPhysics")
        (set `self.fireBoolean` true)
        (`self.fireOn`)
        (else
          (`KismetSystemLibrary.PrintString` "The fire is out of wood"))))))

(event `self.Interact.OnComponentBeginOverlap`
  (params (OverlappedComponent :type "PrimitiveComponent Object Reference") (OtherActor :type "Actor Object Reference") (OtherComp :type "PrimitiveComponent Object Reference") (OtherBodyIndex :type Integer) (bFromSweep :type Boolean) (SweepResult :type "HitResult Structure (by ref)"))
  ;[1 1 1] Add Wood To Fire
  (`self.EnableInput` (`GameplayStatics.GetPlayerController` 0))
  (`KismetSystemLibrary.PrintString` "Press the \"F\" key to add wood"))

(event `Key|F`
  (params (Key :type "Key Structure" :default "AnyKey"))
  ;[1 1 1] Add Wood To Fire
  (:`Pressed`
    (bind _asthird_person_character (cast `/Game/ThirdPersonBP/Blueprints/ThirdPersonCharacter` (`GameplayStatics.GetPlayerCharacter` 0)))
    (bind (_haswood1 _woodamount1) (`self.findWood` (`/Game/Blueprints/BaseInventory.ItemList` (`/Game/ThirdPersonBP/Blueprints/ThirdPersonCharacter.Backpack` _asthird_person_character))))
    (if _haswood1
      (`self.addWood` _woodamount1)
      (else
        (`KismetSystemLibrary.PrintString` "You have no wood")))))

(event `self.Interact.OnComponentEndOverlap`
  (params (OverlappedComponent :type "PrimitiveComponent Object Reference") (OtherActor :type "Actor Object Reference") (OtherComp :type "PrimitiveComponent Object Reference") (OtherBodyIndex :type Integer))
  ;[1 1 1] Add Wood To Fire
  (`self.DisableInput` (`GameplayStatics.GetPlayerController` 0)))

(event `fireOn`
  (bind _firewood (`self.fireWood`))
  ;[1 1 1] Burn Wood
  (bind (_direction _newtrack_0) (`Timeline|BurningWood` :!via `PlayFromStart` :!label _label_2)
    (:`Update`
      (if (`self.fireBoolean`)
        (if (>= _newtrack_0 0.9)
          (if (>= _firewood 1)
            (set `self.fireWood` (- _firewood 1))
            (goto _label_2 :!via `PlayFromStart`)
            (else
              (`self.noWood`))))))))

(fn `addWood`
  (params (woodAmount :type Integer))
  (set `self.fireWood` woodAmount)
  (`KismetSystemLibrary.PrintString` (`KismetStringLibrary.BuildString_Int` "" "+" woodAmount " Wood Added")))

(fn `burnWood`
  (set `self.fireWood` (- (`self.fireWood`) 1)))

(fn `findWood`
  (params (NewParam :type "Array of /Game/Blueprints/InventorySlot Structure"))
  (returns (hasWood1 :type Boolean) (woodAmount1 :type Integer))
  (locals (hasWood :type Boolean) (woodAmount :type Integer))
  (for (_array_element _array_index) NewParam
    (bind (_item _slotcount) (break `/Game/Blueprints/InventorySlot` _array_element))
    (if (== (`/Game/Blueprints/BaseItem.Name` _item) "Wood")
      (set `local.hasWood` true)
      (set `local.woodAmount` (+ _slotcount (`local.woodAmount`)))
      (`KismetArrayLibrary.Array_Remove` NewParam _array_index)
      (break)
      (else
        (set `local.hasWood` false))))
  (return (`local.hasWood`) (+ (`self.fireWood`) (`local.woodAmount`))))

(fn `toggleFire`
  (params (fireStatus :type Boolean)))

(fn `UserConstructionScript`)