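; Day-night cycle Blueprint that drives sun, moon, sky, clock, day count and world temperature from the SunMovement timeline.
; Timeline updates rotate both lights, switch the sun off at night, format hour and minute strings, and set post-process gamma.
; A trigger flags the player indoors, adding warmth to the temperature, more if the first Fire actor is lit.
; Finishing increments Day and replays the timeline, though no event here initially starts it.
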(event `self.ReceiveBeginPlay`
  (set `self.day` 1.0)
  (set `self.inside` false))

(event `self.HouseTempTrigger.OnActorBeginOverlap`
  (params (OverlappedActor :type "Actor Object Reference") (OtherActor :type "Actor Object Reference"))
  (if (`KismetStringLibrary.EqualEqual_StrStr` (`KismetSystemLibrary.GetDisplayName` OtherActor) "ThirdPersonCharacter")
    (set `self.inside` true)))

(event `self.HouseTempTrigger.OnActorEndOverlap`
  (params (OverlappedActor :type "Actor Object Reference") (OtherActor :type "Actor Object Reference"))
  (if (`KismetStringLibrary.EqualEqual_StrStr` (`KismetSystemLibrary.GetDisplayName` OtherActor) "ThirdPersonCharacter")
    (set `self.inside` false)))

(fn `UserConstructionScript`)